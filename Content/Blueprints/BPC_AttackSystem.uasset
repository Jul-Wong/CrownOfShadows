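; Player attack component for BP_ThirdPersonCharacter that runs a sword combo and deals melee damage.
; Attack input plays one of three montages by AttackIndex, buffering presses in SaveAttack for SwordAttackCombo to continue or stop; the fourth kick attack is never called.
; Externally triggered sphere traces (timer-looped blade sweep with hit cooldown, single-shot stab and kick) damage "Damageable" actors with camera shake, sound and blood effects.
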(event Custom|Sword%20Attack
  ;[0.15 0.15 0.15 0.5] Combo System
  ;;[0.15 0.15 0.15 0.5] Sword Attack
  (if (Variables|Default|GetIs%20Attacking)
    (Variables|Default|SetSave%20Attack true)
    (else
      (Variables|Default|SetIs%20Attacking true)
      (switch int (Variables|Default|GetAttack%20Index)
        (:0
          (CallFunction|Attack1))
        (:1
          (CallFunction|Attack2))
        (:2
          (CallFunction|Attack3))))))

(event Custom|Sword%20Attack%20Combo
  ;[0.15 0.15 0.15 0.5] Combo System
  ;;[0.15 0.15 0.15 0.5] Combo Continue
  (if (Variables|Default|GetSave%20Attack)
    (Variables|Default|SetSave%20Attack false)
    (switch int (Variables|Default|GetAttack%20Index)
      (:0
        (CallFunction|Attack1))
      (:1
        (CallFunction|Attack2))
      (:2
        (CallFunction|Attack3)))
    (else
      (CallFunction|StopCombo))))

(event Custom|Attack%202
  ;[0.15 0.15 0.15 0.5] Combo System
  ;;[0.15 0.15 0.15 0.5] Attack 2
  (Utilities|FlowControl|DoOnce false :!label _label
    (:Completed
      (Utilities|FlowControl|Delay 0.1)
      (Animation|Montage|PlayMontage (Variables|Default|GetCharacter%20Mesh) "/Game/Characters/MainCharacter/Animations/SwordAttacks/Attack2_Montage.Attack2_Montage"
        (:then
          (Variables|Default|SetAttack%20Index 2)
          (goto _label Reset))))))

(event Custom|Sphere%20Trace%20Kick
  (bind _character_bp (Variables|Default|GetCharacter%20BP))
  (bind _spheretrace (Variables|/Game/ThirdPerson/Blueprints/BP_ThirdPersonCharacter.BP_ThirdPersonCharacter_C|GetSphereTrace _character_bp))
  (bind _returnvalue (Transformation|GetWorldLocation _spheretrace))
  ;[0.15 0.15 0.15 0.5] Sphere Trace (Kick)
  (bind (_outhit _returnvalue_2) (Collision|SphereTraceByChannel _returnvalue _returnvalue 25.0 "TraceTypeQuery1" false 0 "None" true "(R=1.000000,G=0.000000,B=0.000000,A=1.000000)" "(R=0.000000,G=1.000000,B=0.000000,A=1.000000)" 0.1))
  (if _returnvalue_2
    (if (Actor|ActorHasTag (.HitActor (Collision|BreakHitResult _outhit)) "Damageable")
      (Game|Damage|ApplyDamage (.HitActor (Collision|BreakHitResult _outhit)) 1e+01 0 0)
      (Camera|PlayWorldCameraShake "/Game/Blueprints/BP_SwordHitCameraShake.BP_SwordHitCameraShake_C" (.Location (Collision|BreakHitResult _outhit)) 0.0 2e+03)
      (CallFunction|PlaySwordHitsSound)
      (Effects|SpawnEmitteratLocation "/Game/Effects/Particles/Blood/P_Blood_Splat_Cone.P_Blood_Splat_Cone" (.Location (Collision|BreakHitResult _outhit)) (Math|Rotator|MakeRotfromXY (.Normal (Collision|BreakHitResult _outhit)) (.Normal (Collision|BreakHitResult _outhit))) "0.400000,0.400000,0.400000" true "AutoRelease"))))

(event Custom|Attack%203
  ;[0.15 0.15 0.15 0.5] Combo System
  ;;[0.15 0.15 0.15 0.5] Attack 3
  (Utilities|FlowControl|DoOnce false :!label _label
    (:Completed
      (Utilities|FlowControl|Delay 0.1)
      (Animation|Montage|PlayMontage (Variables|Default|GetCharacter%20Mesh) "/Game/Characters/MainCharacter/Animations/SwordAttacks/Attack3_Montage.Attack3_Montage"
        (:then
          (Variables|Default|SetAttack%20Index 3)
          (goto _label Reset))))))

(event Custom|Stop%20Combo
  ;[0.15 0.15 0.15 0.5] Combo System
  ;;[0.15 0.15 0.15 0.5] Stop Attack/Combo
  (Variables|Default|SetIs%20Attacking false)
  (Variables|Default|SetAttack%20Index 0))

(event Custom|Attack%204
  ;[0.15 0.15 0.15 0.5] Combo System
  ;;[0.15 0.15 0.15 0.5] Attack 4
  (Utilities|FlowControl|DoOnce false :!label _label
    (:Completed
      (Utilities|FlowControl|Delay 0.1)
      (Animation|Montage|PlayMontage (Variables|Default|GetCharacter%20Mesh) "/Game/Characters/MainCharacter/Animations/SwordAttacks/Kick_Montage.Kick_Montage"
        (:then
          (Variables|Default|SetAttack%20Index 4)
          (goto _label Reset))))))

(event Custom|Attack%201
  ;[0.15 0.15 0.15 0.5] Combo System
  ;;[0.15 0.15 0.15 0.5] Attack 1
  (Utilities|FlowControl|DoOnce false :!label _label
    (:Completed
      (Utilities|FlowControl|Delay 0.1)
      (Animation|Montage|PlayMontage (Variables|Default|GetCharacter%20Mesh) "/Game/Characters/MainCharacter/Animations/SwordAttacks/Attack1_Montage.Attack1_Montage"
        (:then
          (Variables|Default|SetAttack%20Index 1)
          (goto _label Reset))))))

(event Custom|Start%20Sword%20Trace
  ;[0.15 0.15 0.15 0.5] Sword Trace
  (bind _returnvalue (Utilities|Time|SetTimerbyEvent (delegate Custom|Sword%20Trace%20Loop) 0.01 true))
  (Variables|Default|SetSwordTraceLoop _returnvalue))

(event Custom|Sword%20Trace%20Loop
  (bind _character_bp (Variables|Default|GetCharacter%20BP))
  ;[0.15 0.15 0.15 0.5] Sword Trace
  (bind (_outhit _returnvalue) (Collision|SphereTraceByChannel (Transformation|GetWorldLocation (Variables|/Game/ThirdPerson/Blueprints/BP_ThirdPersonCharacter.BP_ThirdPersonCharacter_C|GetSwordTopPoint _character_bp)) (Transformation|GetWorldLocation (Variables|/Game/ThirdPerson/Blueprints/BP_ThirdPersonCharacter.BP_ThirdPersonCharacter_C|GetSwordBottomPoint _character_bp)) 1e+01 "TraceTypeQuery1" false 0 "None" true "(R=1.000000,G=0.000000,B=0.000000,A=1.000000)" "(R=0.000000,G=1.000000,B=0.000000,A=1.000000)" 0.2))
  (if _returnvalue
    (if (Actor|ActorHasTag (.HitActor (Collision|BreakHitResult _outhit)) "Damageable")
      (Utilities|FlowControl|DoOnce false :!label _label
        (:Completed
          (Game|Damage|ApplyDamage (.HitActor (Collision|BreakHitResult _outhit)) 1e+01 0 0)
          (Camera|PlayWorldCameraShake "/Game/Blueprints/BP_SwordHitCameraShake.BP_SwordHitCameraShake_C" (.Location (Collision|BreakHitResult _outhit)) 0.0 2e+03)
          (CallFunction|PlaySwordHitsSound)
          (Effects|SpawnEmitteratLocation "/Game/Effects/Particles/Blood/P_Blood_Splat_Cone.P_Blood_Splat_Cone" (.Location (Collision|BreakHitResult _outhit)) (Math|Rotator|MakeRotfromXY (.Normal (Collision|BreakHitResult _outhit)) (.Normal (Collision|BreakHitResult _outhit))) "0.400000,0.400000,0.400000" true "AutoRelease")
          (Utilities|FlowControl|Delay 0.5)
          (goto _label Reset))))))

(event Custom|Stop%20Sword%20Trace
  ;[0.15 0.15 0.15 0.5] Sword Trace
  (Utilities|Time|ClearandInvalidateTimerbyHandle (Variables|Default|GetSwordTraceLoop)))

(event Custom|Sphere%20Trace%20Stab
  (bind _character_bp (Variables|Default|GetCharacter%20BP))
  ;[0.15 0.15 0.15 0.5] Sphere Trace (Stab)
  (bind (_outhit _returnvalue) (Collision|SphereTraceByChannel (Transformation|GetWorldLocation (Variables|/Game/ThirdPerson/Blueprints/BP_ThirdPersonCharacter.BP_ThirdPersonCharacter_C|GetSphereTraceStart _character_bp)) (Transformation|GetWorldLocation (Variables|/Game/ThirdPerson/Blueprints/BP_ThirdPersonCharacter.BP_ThirdPersonCharacter_C|GetSphereTraceEnd _character_bp)) 25.0 "TraceTypeQuery1" false 0 "None" true "(R=1.000000,G=0.000000,B=0.000000,A=1.000000)" "(R=0.000000,G=1.000000,B=0.000000,A=1.000000)" 0.1))
  (if _returnvalue
    (if (Actor|ActorHasTag (.HitActor (Collision|BreakHitResult _outhit)) "Damageable")
      (Game|Damage|ApplyDamage (.HitActor (Collision|BreakHitResult _outhit)) 1e+01 0 0)
      (Camera|PlayWorldCameraShake "/Game/Blueprints/BP_SwordHitCameraShake.BP_SwordHitCameraShake_C" (.Location (Collision|BreakHitResult _outhit)) 0.0 2e+03)
      (CallFunction|PlaySwordHitsSound)
      (Effects|SpawnEmitteratLocation "/Game/Effects/Particles/Blood/P_Blood_Splat_Cone.P_Blood_Splat_Cone" (.Location (Collision|BreakHitResult _outhit)) (Math|Rotator|MakeRotfromXY (.Normal (Collision|BreakHitResult _outhit)) (.Normal (Collision|BreakHitResult _outhit))) "0.400000,0.400000,0.400000" true "AutoRelease"))))

(event Custom|Play%20Sword%20Hits%20Sound
  ;[0.15 0.15 0.15 0.5] Play Sword Hit Sounds
  (Audio|PlaySoundatLocation "/Game/Audio/Sword_Hits/MS_Sword_Hit.MS_Sword_Hit" (Transformation|GetActorLocation (Components|GetOwner)) "0, 0, 0" 1.0 1.0 0.0 0 0 0 0))

(event Input|EnhancedActionEvents|EnhancedInputActionIA_Attack
  (params (ActionValue :type Boolean) (ElapsedSeconds :type Float%20%28double-precision%29) (TriggeredSeconds :type Float%20%28double-precision%29) (InputAction :type Input%20Action%20Object%20Reference :default "/Game/Input/Actions/IA_Attack.IA_Attack"))
  ;[0.15 0.15 0.15 0.5] Combo System
  ;;[0.15 0.15 0.15 0.5] Attack Input
  (:Started
    (if (Variables|Default|GetCan%20Attack)
      (CallFunction|SwordAttack))))

(event EventBeginPlay
  ;[0.15 0.15 0.15 0.5] Combo System
  ;;[0.15 0.15 0.15 0.5] Cast Player Mesh
  (bind _asbp_third_person_character (Utilities|Casting|CastToBP_ThirdPersonCharacter (Components|GetOwner)))
  (Variables|Default|SetCharacter%20BP _asbp_third_person_character)
  (Variables|Default|SetCharacter%20Mesh (Variables|/Script/Engine.Character|GetMesh _asbp_third_person_character)))