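; Quest giver actor that the player interacts with to read dialogue and then view its list of quests.
; An interact prompt widget shows while the player is inside the trigger radius and turns to face the camera each tick.
; Each interaction advances the dialogue array; after the last line, it opens a quest widget filled from the Quests array.
; Interacting again or calling CloseWidget removes that widget and restores game-only input.
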(event OnComponentBeginOverlap(TriggerRadius)
  (params (OverlappedComponent :type Primitive%20Component%20Object%20Reference) (OtherActor :type Actor%20Object%20Reference) (OtherComp :type Primitive%20Component%20Object%20Reference) (OtherBodyIndex :type Integer) (bFromSweep :type Boolean) (SweepResult :type Hit%20Result%20Structure%20%28by%20ref%29))
  (Utilities|Casting|CastToBP_ThirdPersonCharacter OtherActor)
  (Rendering|SetVisibility (Variables|Default|GetInteract%20Widget) true false))

(event OnComponentEndOverlap(TriggerRadius)
  (params (OverlappedComponent :type Primitive%20Component%20Object%20Reference) (OtherActor :type Actor%20Object%20Reference) (OtherComp :type Primitive%20Component%20Object%20Reference) (OtherBodyIndex :type Integer))
  (Utilities|Casting|CastToBP_ThirdPersonCharacter OtherActor)
  (Rendering|SetVisibility (Variables|Default|GetInteract%20Widget) false false))

(event Custom|Close%20Widget
  (bind _returnvalue (Game|GetPlayerController 0))
  (Widget|RemovefromParent (Variables|Default|GetQuest%20Widget))
  (Variables|Default|SetQuest%20Widget 0)
  (Variables|/Script/Engine.PlayerController|SetbShowMouseCursor _returnvalue false)
  (Input|SetInputModeGameOnly _returnvalue false)
  (Variables|Default|SetWidget%20Active false))

(event Custom|Open%20Quests%20Widget
  (bind _returnvalue (UserInterface|CreateWidget "/Game/Quest_System/WB_Quest_Giver.WB_Quest_Giver_C"))
  (bind _output_get (Variables|Default|SetQuest%20Widget _returnvalue))
  (UserInterface|Viewport|AddtoViewport _output_get 0)
  (Variables|Default|SetWidget%20Active true)
  (Variables|/Game/Quest_System/WB_Quest_Giver.WB_Quest_Giver_C|SetQuest%20Giver%20BP (Variables|Default|GetQuest%20Widget) self)
  (for _array_element (Variables|Default|GetQuests)
    (Default|AddQuest (Variables|Default|GetQuest%20Widget) _array_element)))

(event EventTick
  (params (DeltaSeconds :type Float%20%28single-precision%29))
  (Transformation|SetWorldRotation (Variables|Default|GetInteract%20Widget) (Math|Rotator|FindLookatRotation (Transformation|GetWorldLocation (Variables|Default|GetInteract%20Widget)) (Transformation|GetWorldLocation (Variables|/Script/Engine.PlayerCameraManager|GetTransformComponent (Game|GetPlayerCameraManager 0)))) false false))

(event EventInteract
  (bind _returnvalue (Game|GetPlayerController 0))
  (bind _returnvalue_2 (Game|GetPlayerController 0))
  (if (not (Variables|Default|GetWidget%20Active))
    (if (not (Variables|Default|GetDialogue%20Opened))
      (bind _returnvalue_3 (UserInterface|CreateWidget "/Game/Quest_System/WB_Quest_Giver_Dialogue.WB_Quest_Giver_Dialogue_C"))
      (Variables|Default|SetDialogue%20Widget _returnvalue_3)
      (UserInterface|Viewport|AddtoViewport _returnvalue_3 0)
      (Variables|Default|SetDialogue%20Opened true)
      (Rendering|Components|TextRender|SetText (Variables|/Game/Quest_System/WB_Quest_Giver_Dialogue.WB_Quest_Giver_Dialogue_C|GetDialogueText (Variables|Default|GetDialogue%20Widget)) (Utilities|Text|ToText(String) (Utilities|Array|Get(acopy) (Variables|Default|GetDialogue) (Variables|Default|GetDialogue%20Index))))
      (Math|Integer|IncrementInt (Variables|Default|GetDialogue%20Index)
        (:%20%20
          (Variables|/Script/Engine.PlayerController|SetbShowMouseCursor _returnvalue_2 true)
          (Input|SetInputModeGameandUI _returnvalue_2 (Variables|Default|GetQuest%20Widget) "DoNotLock" true false)))
      (else
        (Rendering|Components|TextRender|SetText (Variables|/Game/Quest_System/WB_Quest_Giver_Dialogue.WB_Quest_Giver_Dialogue_C|GetDialogueText (Variables|Default|GetDialogue%20Widget)) (Utilities|Text|ToText(String) (Utilities|Array|Get(acopy) (Variables|Default|GetDialogue) (Variables|Default|GetDialogue%20Index))))
        (Math|Integer|IncrementInt (Variables|Default|GetDialogue%20Index)
          (:%20%20
            (if (> (Variables|Default|GetDialogue%20Index) (Utilities|Array|Length (Variables|Default|GetDialogue)))
              (Widget|RemovefromParent (Variables|Default|GetDialogue%20Widget))
              (Variables|Default|SetDialogue%20Widget 0)
              (Variables|Default|SetDialogue%20Index 0)
              (Variables|Default|SetDialogue%20Opened false)
              (CallFunction|OpenQuestsWidget))))))
    (else
      (Widget|RemovefromParent (Variables|Default|GetQuest%20Widget))
      (Variables|Default|SetQuest%20Widget 0)
      (Variables|/Script/Engine.PlayerController|SetbShowMouseCursor _returnvalue false)
      (Input|SetInputModeGameOnly _returnvalue false)
      (Variables|Default|SetWidget%20Active false))))

(fn ConstructionScript)