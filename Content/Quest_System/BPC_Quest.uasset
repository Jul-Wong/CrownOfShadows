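; Quest component that tracks the active quest, updates the quest HUD widget and awards XP on completion.
; It creates the HUD on BeginPlay and exposes events to show the quest and its objectives.
; Enemy elimination, chest opening and button press events mark matching objectives complete and increment a counter.
; When the counter reaches the objective count, it plays the completion animation, grants XP through the player's stats component and clears the quest.
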(event Custom|Set%20Active%20Quest%20Text
  (Rendering|Components|TextRender|SetText (Variables|/Game/Quest_System/WB_QuestHUD.WB_QuestHUD_C|GetActiveQuestText (Variables|Default|GetQuest%20HUD%20Widget)) (Utilities|Text|ToText(Name) (.Name (Utilities|Struct|BreakS_Quest (Variables|Default|GetActive%20Quest)))))
  (Default|ShowQuestPanel (Variables|Default|GetQuest%20HUD%20Widget)))

(event Custom|Set%20Objectives
  (Default|FillObjectives (Variables|Default|GetQuest%20HUD%20Widget) (.objectives (Variables|Default|GetActive%20Quest))))

(event Custom|Eliminate%20Enemy
  (params (Enemy%20Eliminated :type Actor%20Object%20Reference))
  ;[0.15 0.15 0.15 0.5] Eliminate Enemy Objective
  (for _array_element (.objectives (Variables|Default|GetActive%20Quest))
    (if (and (not (.Complete (Utilities|Struct|BreakS_Quest_Objectives _array_element))) (.IsEliminateEnemyObjective (Utilities|Struct|BreakS_Quest_Objectives _array_element)))
      (if (!= (Utilities|Array|Length (Variables|Default|GetEnemy%20Actors%20Array)) 0)
        _
        (else
          (bind _output_get (Variables|Default|SetEnemy%20Actors%20Array (.ActorstoEliminate (Utilities|Struct|BreakS_Quest_Objectives _array_element))))))
      (Utilities|Array|RemoveItem _output_get Enemy%20Eliminated)
      (|SetBy-RefVar _array_element (Utilities|Struct|MakeS_Quest_Objectives (.Name (Utilities|Struct|BreakS_Quest_Objectives _array_element)) false (Variables|Default|GetEnemy%20Actors%20Array) 0 (.IsEliminateEnemyObjective (Utilities|Struct|BreakS_Quest_Objectives _array_element)) false false 0))
      (Development|PrintString (Utilities|String|ToString(Integer) (Utilities|Array|Length (Variables|Default|GetEnemy%20Actors%20Array))))
      (if (== (Utilities|Array|Length (Variables|Default|GetEnemy%20Actors%20Array)) 0)
        (|SetBy-RefVar _array_element (Utilities|Struct|MakeS_Quest_Objectives (.Name (Utilities|Struct|BreakS_Quest_Objectives _array_element)) true 0 0 (.IsEliminateEnemyObjective (Utilities|Struct|BreakS_Quest_Objectives _array_element)) false false 0))
        (Default|CompleteObjective (Variables|Default|GetQuest%20HUD%20Widget) _array_element)
        (CallFunction|ObjectiveComplete)))))

(event Custom|Open%20Chest
  (params (Chest :type Actor%20Object%20Reference))
  (bind _active_quest (Variables|Default|GetActive%20Quest))
  ;[0.15 0.15 0.15 0.5] Open Chest Objective
  (for _array_element (.objectives _active_quest)
    (if (and (.IsChestObjective (Utilities|Struct|BreakS_Quest_Objectives _array_element)) (== (.ChesttoOpen (Utilities|Struct|BreakS_Quest_Objectives _array_element)) Chest))
      (|SetBy-RefVar _array_element (Utilities|Struct|MakeS_Quest_Objectives (.name _active_quest) true 0 0 false (.IsChestObjective (Utilities|Struct|BreakS_Quest_Objectives _array_element)) false 0))
      (Default|CompleteObjective (Variables|Default|GetQuest%20HUD%20Widget) _array_element)
      (CallFunction|ObjectiveComplete))))

(event Custom|Objective%20Complete
  ;[0.15 0.15 0.15 0.5] Complete Objective
  (Math|Integer|IncrementInt (Variables|Default|GetObjectives%20Completed)
    (:%20%20
      (if (>= (Variables|Default|GetObjectives%20Completed) (Utilities|Array|Length (.objectives (Variables|Default|GetActive%20Quest))))
        (Variables|Default|SetActive%20Quest (Utilities|Struct|MakeS_Quest (.name (Variables|Default|GetActive%20Quest)) (.description (Variables|Default|GetActive%20Quest)) (.sidequest (Variables|Default|GetActive%20Quest)) true (.objectives (Variables|Default|GetActive%20Quest)) (.xpreward (Variables|Default|GetActive%20Quest)) false))
        (Utilities|FlowControl|DoOnce false :!label _label
          (:Completed
            (Default|PlayQuestCompletedAnimation (Variables|Default|GetQuest%20HUD%20Widget))
            (bind _asbp_third_person_character (Utilities|Casting|CastToBP_ThirdPersonCharacter (Game|GetPlayerCharacter 0)))
            (Default|IncreaseXP (Variables|/Game/ThirdPerson/Blueprints/BP_ThirdPersonCharacter.BP_ThirdPersonCharacter_C|GetBPC_PlayerStats _asbp_third_person_character) (.xpreward (Variables|Default|GetActive%20Quest)))
            (Variables|Default|SetActive%20Quest "")
            (Variables|Default|SetObjectives%20Completed 0)
            (goto _label Reset)))))))

(event Custom|Button%20Press%20Event
  (params (Quest :type S%20Quest%20Structure) (Input%20Key :type Input%20Action%20Object%20Reference))
  ;[0.15 0.15 0.15 0.5] Press Button Event Quest
  (for _array_element (.Objectives (Utilities|Struct|BreakS_Quest Quest))
    (if (Math|Boolean|ANDBoolean (not (.Complete (Utilities|Struct|BreakS_Quest_Objectives _array_element))) (.IsButtonPressObjective (Utilities|Struct|BreakS_Quest_Objectives _array_element)) (== (.ButtonToPress (Utilities|Struct|BreakS_Quest_Objectives _array_element)) Input%20Key))
      (|SetBy-RefVar _array_element (Utilities|Struct|MakeS_Quest_Objectives (.Name (Utilities|Struct|BreakS_Quest_Objectives _array_element)) true 0 0 false false (.IsButtonPressObjective (Utilities|Struct|BreakS_Quest_Objectives _array_element)) (.ButtonToPress (Utilities|Struct|BreakS_Quest_Objectives _array_element))))
      (Default|CompleteObjective (Variables|Default|GetQuest%20HUD%20Widget) _array_element)
      (CallFunction|ObjectiveComplete))))

(event EventBeginPlay
  (bind _returnvalue (UserInterface|CreateWidget "/Game/Quest_System/WB_QuestHUD.WB_QuestHUD_C"))
  (bind _output_get (Variables|Default|SetQuest%20HUD%20Widget _returnvalue))
  (UserInterface|Viewport|AddtoViewport _output_get 0)
  (Default|HideQuestPanel (Variables|Default|GetQuest%20HUD%20Widget)))

(event Input|KeyboardEvents|DebugKeyU
  (params (Key :type Key%20Structure :default "None") (ActionValue :type Input%20Action%20Value%20Structure))
  (bind _active_quest (Variables|Default|GetActive%20Quest))
  (bind (_name _description _sidequest _completed _objectives) (Utilities|Struct|BreakS_Quest _active_quest))
  (:Pressed
    (Development|PrintString (Utilities|String|ToString(Name) _name) true true "(R=0.577580,G=0.212231,B=0.947307,A=1.000000)")
    (Development|PrintString (Utilities|String|ToString(Boolean) _completed) true true "(R=0.291771,G=0.000000,B=0.000000,A=1.000000)")
    (Development|PrintString (Utilities|String|ToString(Integer) (Utilities|Array|Length _objectives)))
    (Development|PrintString (Utilities|String|ToString(Integer) (Variables|Default|GetObjectives%20Completed)) true true "(R=0.965162,G=1.000000,B=0.841192,A=1.000000)")))